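; BP_Plantation is a procedural scatter actor that fills a box area with instanced meshes, placed when its construction script runs.
; It creates an instanced static mesh component per active mesh entry, with optional collision, and reads the box bounds.
; For each Density iteration, it picks a random component and XY point, line-traces vertically for the floor, then adds a scaled instance sunk by Depression.
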(event EventBeginPlay)

(event Collision|EventActorBeginOverlap
  (params (OtherActor :type Actor%20Object%20Reference)))

(event EventTick
  (params (DeltaSeconds :type Float%20%28single-precision%29)))

(fn ConstructionScript
  (Utilities|FlowControl|Sequence
    (:then_0
      (CallFunction|SetMeshesIntances))
    (:then_1
      (CallFunction|SetBoxBounds))
    (:then_2
      (CallFunction|InstantiateMesh))))

(fn SetMeshesIntances
  (for _array_element (Variables|EditableParameters|GetActive%20Mesh)
    (if (.active _array_element)
      (bind _returnvalue (AddComponent|AddInstancedStaticMeshComponent false))
      (Components|StaticMesh|SetStaticMesh _returnvalue (.mesh _array_element))
      (Utilities|Array|Add (Variables|Generation|GetInstancied%20Static%20mesh) _returnvalue)
      (if (Variables|EditableParameters|GetCollisionEnable)
        (Collision|SetCollisionEnabled _returnvalue "QueryAndPhysics")
        (else
          (Collision|SetCollisionEnabled _returnvalue "NoCollision"))))))

(fn SetBoxBounds
  (bind _box (Variables|Default|GetBox))
  (bind (_origin _boxextent) (Collision|GetComponentBounds _box))
  (Variables|Generation|SetBoxOrigin _origin)
  (Variables|Generation|SetBoxExtent _boxextent))

(fn InstantiateMesh
  (bind _boxorigin (Variables|Generation|GetBoxOrigin))
  (bind _boxextent (Variables|Generation|GetBoxExtent))
  (bind _instancied_static_mesh (Variables|Generation|GetInstancied%20Static%20mesh))
  (bind _returnvalue (Math|Random|RandomPointinBoundingBox _boxorigin _boxextent))
  (bind (_x _y) (Math|Vector|BreakVector _returnvalue))
  (for _index (range 0 (Variables|EditableParameters|GetDensity))
    (bind _newposition (CallFunction|GetPositiononFloor (Math|Vector|MakeVector _x _y 0.0)))
    (Class|InstancedStaticMeshComponent|AddInstanceWorldSpace (Utilities|Array|Get(acopy) _instancied_static_mesh (Math|Random|RandomIntegerinRange 0 (- (Utilities|Array|Length _instancied_static_mesh) 1))) (Math|Transform|MakeTransform _newposition (Math|Rotator|MakeRotator 0.0 0.0 (Math|Random|RandomFloat)) (Variables|EditableParameters|GetSize)))))

(fn GetPositiononFloor
  (params (BasePoint :type Vector))
  (bind _outhit (Collision|LineTraceForObjects (- BasePoint "0, 0,10000000.000000") (+ BasePoint "0, 0,10000000.000000") (Variables|Generation|GetRaycastTypes) false 0 "None"))
  (return (Math|Vector|MakeVector (.x (.location _outhit)) (.y (.location _outhit)) (- (.z (.location _outhit)) (Variables|EditableParameters|GetDepression)))))