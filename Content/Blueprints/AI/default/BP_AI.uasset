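; Base AI enemy character that damages the first-person player on hit, optionally launches them, and awards points when it dies.
; Taking damage reduces health, plays a sound and starts temporary invincibility, during which the mesh blinks.
; Tick drives delay-based timers that clear invincibility and re-arm knockback.
; Walk and Run events switch movement speed, and player overlap plays a damage sound.
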(event Custom|Walk
  (Variables|/Script/Engine.CharacterMovementComponent|SetMaxWalkSpeed (Variables|Character|GetCharacterMovement) (Variables|AI|Speed|GetWalkingSpeed)))

(event Custom|Run
  (Variables|/Script/Engine.CharacterMovementComponent|SetMaxWalkSpeed (Variables|Character|GetCharacterMovement) (Variables|AI|Speed|GetRunningSpeed)))

(event EventTick
  (params (DeltaSeconds :type Float%20%28single-precision%29))
  (Utilities|FlowControl|Sequence
    (:then_0
      (|ProcessInvicibilityChecking))
    (:then_1
      (|ProcessKnockBackChecking))))

(event Game|Damage|EventAnyDamage
  (params (Damage :type Float%20%28single-precision%29) (DamageType :type Damage%20Type%20Object%20Reference) (InstigatedBy :type Controller%20Object%20Reference) (DamageCauser :type Actor%20Object%20Reference))
  (CallFunction|GetDamaged Damage))

(event Collision|EventHit
  (params (MyComp :type Primitive%20Component%20Object%20Reference) (Other :type Actor%20Object%20Reference) (OtherComp :type Primitive%20Component%20Object%20Reference) (bSelfMoved :type Boolean) (HitLocation :type Vector :default "0, 0, 0") (HitNormal :type Vector :default "0, 0, 0") (NormalImpulse :type Vector :default "0, 0, 0") (Hit :type Hit%20Result%20Structure%20%28by%20ref%29))
  (Utilities|FlowControl|Sequence
    (:then_0
      (CallFunction|KnockBack Other))
    (:then_1
      (CallFunction|ApplyDamages Other))))

(event Collision|EventActorBeginOverlap
  (params (OtherActor :type Actor%20Object%20Reference))
  (Utilities|Casting|CastToFirstPersonCharacter OtherActor)
  (Audio|PlaySoundatLocation (Variables|AI|Damages|GetDamageSound) (Transformation|GetActorLocation) "0, 0, 0" 1.0 1.0 0.0 0 0 0))

(fn ConstructionScript)

(fn GetDamaged
  (params (Damages :type Float%20%28single-precision%29))
  (if (not (Variables|AI|Health|GetIsInvicible))
    (Variables|AI|Health|SetHealthPoints (- (Variables|AI|Health|GetHealthPoints) Damages))
    (Variables|AI|Health|SetIsInvicible true)
    (Audio|PlaySoundatLocation (Variables|AI|Health|GetgetDamagedSound) (Transformation|GetActorLocation) "0, 0, 0" 1.0 1.0 0.0 0 0 0)
    (if (<= (Variables|AI|Health|GetHealthPoints) 0.0)
      (CallFunction|Die))))

(fn KnockBack
  (params (OtherActor :type Actor%20Object%20Reference))
  (if (Variables|AI|Damages|GethasKnockBack)
    (if (Variables|AI|Damages|GetCanKnockBack)
      (bind _asfirst_person_character (Utilities|Casting|CastToFirstPersonCharacter OtherActor))
      (Character|LaunchCharacter _asfirst_person_character (Variables|AI|Damages|GetKnockEjection) false false)
      (Variables|AI|Damages|SetCanKnockBack false))))

(fn ApplyDamages
  (params (OtherActor :type Actor%20Object%20Reference))
  (if (Variables|AI|Damages|GetCanDamage)
    (bind _asfirst_person_character (Utilities|Casting|CastToFirstPersonCharacter OtherActor))
    (Game|Damage|ApplyDamage _asfirst_person_character (Variables|AI|Damages|GetDamages) 0 0)))

(fn Die
  (Utilities|FlowControl|DoOnce false
    (:Completed
      (Actor|DestroyActor)
      (bind _asfirst_person_character (Utilities|Casting|CastToFirstPersonCharacter (Game|GetPlayerCharacter 0)))
      (Default|GainPoints _asfirst_person_character (Variables|AI|GetPoints)))))