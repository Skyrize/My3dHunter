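; AI spawner actor that periodically spawns a configurable pawn class at random points inside its box bounds.
; A Delay on Tick paces spawning, using a start delay for the first spawn and a between-spawn delay afterwards via a DoOnce.
; Each cycle spawns only while the count of all actors of that class in the level is below the maximum, ignoring collision failure.
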(event EventTick
  (params (DeltaSeconds :type Float%20%28single-precision%29))
  (bind _box (Variables|Default|GetBox))
  (bind (_origin _boxextent) (Collision|GetComponentBounds _box))
  (Utilities|FlowControl|Delay (Variables|Settings|GetSpawnDelay))
  (Utilities|FlowControl|Sequence
    (:then_0
      (bind _outactors (Actor|GetAllActorsOfClass (Variables|Settings|GetSpawnedEntity)))
      (if (< (Utilities|Array|Length _outactors) (Variables|Settings|GetMaxEntities))
        (bind _aspawn (Utilities|Casting|CastToPawnClass (Variables|Settings|GetSpawnedEntity)))
        (AI|SpawnAIFromClass _aspawn 0 (Math|Random|RandomPointinBoundingBox _origin _boxextent) "0, 0, 0" true)))
    (:then_1
      (Utilities|FlowControl|DoOnce false
        (:Completed
          (Variables|Settings|SetSpawnDelay (Variables|Settings|GetBetweenSpawnDelay)))))))

(event EventBeginPlay
  (Variables|Settings|SetSpawnDelay (Variables|Settings|GetStartDelay)))

(fn ConstructionScript)