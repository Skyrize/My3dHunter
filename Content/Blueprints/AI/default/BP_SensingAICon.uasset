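; BP_SensingAICon is an AI controller that runs a behavior tree for BP_AI pawns and tracks whether they perceive the player.
; On BeginPlay it sets up the blackboard and starts the behavior tree.
; Perception updates for the FirstPersonCharacter write the sensed state to the CanSeePlayer blackboard key.
; On possession it caches the BP_AI pawn and forwards its Walk and Run events to that pawn.
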(event OnTargetPerceptionUpdated(AIPerception)
  (params (Actor :type Actor%20Object%20Reference) (Stimulus :type AI%20Stimulus%20Structure))
  (Utilities|Casting|CastToFirstPersonCharacter Actor)
  (AI|Components|Blackboard|SetValueasBool (AI|GetBlackboard self) (Variables|Default|GetCanSeePlayer) (.bSuccessfullySensed (Utilities|Struct|BreakAIStimulus Stimulus))))

(event Custom|Run
  (Default|Run (Variables|Default|GetAIPawnRef)))

(event Custom|Walk
  (Default|Walk (Variables|Default|GetAIPawnRef)))

(event EventBeginPlay
  (Class|AIController|UseBlackboard (Variables|Default|GetBlackboardAsset))
  (AI|RunBehaviorTree (Variables|Default|GetBehaviorTree)))

(event EventOnPossess
  (params (PossessedPawn :type Pawn%20Object%20Reference))
  (bind _asbp_ai (Utilities|Casting|CastToBP_AI PossessedPawn))
  (Variables|Default|SetAIPawnRef _asbp_ai))

(fn ConstructionScript)