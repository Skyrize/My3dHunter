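; BP_BirdSpawn is a spawner that keeps the level populated with BP_Bird AI, placing them at random points and yaws within its Box component.
; Tick drives two Delay loops: every ten seconds it counts birds level-wide and resets a DoN gate when few remain.
; The half-second loop feeds that gate, so birds spawn one at a time in capped batches, ignoring collision.
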(event EventTick
  (params (DeltaSeconds :type Float%20%28single-precision%29))
  (bind _box (Variables|Default|GetBox))
  (bind _returnvalue (Components|Box|GetScaledBoxExtent _box))
  (bind (_x _y _z) (Math|Vector|BreakVector _returnvalue))
  (Utilities|FlowControl|Sequence
    (:then_0
      (Utilities|FlowControl|Delay 1e+01)
      (bind _outactors (Actor|GetAllActorsOfClass "/Game/Blueprints/AI/bird/BP_Bird.BP_Bird_C"))
      (if (<= (Utilities|Array|Length _outactors) 8)
        (goto _label Reset)))
    (:then_1
      (Utilities|FlowControl|Delay 0.5)
      (Utilities|FlowControl|DoN 10 :!label _label
        (:Exit
          (AI|SpawnAIFromClass "/Game/Blueprints/AI/bird/BP_Bird.BP_Bird_C" 0 (+ (Math|Vector|MakeVector (Math|Random|RandomFloatinRange (* _x -1.0) _x) (Math|Random|RandomFloatinRange (* _y -1.0) _y) (Math|Random|RandomFloatinRange (* _z -1.0) _z)) (Transformation|GetActorLocation)) (Math|Rotator|MakeRotator 0.0 0.0 (Math|Random|RandomFloatinRange 0.0 359.0)) true))))))

(fn ConstructionScript)