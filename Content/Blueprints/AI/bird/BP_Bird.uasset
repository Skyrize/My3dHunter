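; BP_Bird is a shootable-style AI bird that flies between random points inside BP_Cage volumes and awards HUD points when killed.
; Once Fly is called, a timeline lerps it to its destination with an alternating sideways X offset, facing its motion, then picks another cage's point and repeats.
; Damage plays a sound and drains Health until the bird is destroyed.
; A dynamic material carries its color, adjustable through ChangeColor.
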(event Custom|Fly
  (if (== (Variables|Default|Getreverse) 1)
    (Variables|Default|Setreverse -1)
    (bind (_direction _alpha _birdxoffset) (Timeline|FlyTo PlayFromStart)
      (:Update
        (Transformation|SetActorLocationAndRotation (Math|Vector|MakeVector (+ (* (Variables|Default|Getreverse) _birdxoffset) (.X (Math|Vector|BreakVector (Math|Vector|Lerp(Vector) (Variables|Default|GetHomeLocation) (Variables|Default|GetDestination) _alpha)))) (.Y (Math|Vector|BreakVector (Math|Vector|Lerp(Vector) (Variables|Default|GetHomeLocation) (Variables|Default|GetDestination) _alpha))) (.Z (Math|Vector|BreakVector (Math|Vector|Lerp(Vector) (Variables|Default|GetHomeLocation) (Variables|Default|GetDestination) _alpha)))) (Math|Rotator|MakeRotfromX (- (Math|Vector|MakeVector (+ (* (Variables|Default|Getreverse) _birdxoffset) (.X (Math|Vector|BreakVector (Math|Vector|Lerp(Vector) (Variables|Default|GetHomeLocation) (Variables|Default|GetDestination) _alpha)))) (.Y (Math|Vector|BreakVector (Math|Vector|Lerp(Vector) (Variables|Default|GetHomeLocation) (Variables|Default|GetDestination) _alpha))) (.Z (Math|Vector|BreakVector (Math|Vector|Lerp(Vector) (Variables|Default|GetHomeLocation) (Variables|Default|GetDestination) _alpha)))) (Transformation|GetActorLocation)))))
      (:Finished
        (CallFunction|FindDestination)
        (CallFunction|Fly)))
    (else
      (Variables|Default|Setreverse 1)
      (Timeline|FlyTo PlayFromStart))))

(event EventBeginPlay
  (Utilities|FlowControl|Sequence
    (:then_0
      (Variables|Default|SetCage (Math|Random|RandomIntegerinRange 0 1)))
    (:then_1
      (if (== (Math|Random|RandomIntegerinRange 0 1) 0)
        (Variables|Default|Setreverse -1)
        (else
          (Variables|Default|Setreverse 1))))
    (:then_2
      (bind _outactors (Actor|GetAllActorsOfClass "/Game/Blueprints/AI/bird/BP_Cage.BP_Cage_C"))
      (Variables|Default|SetCages _outactors))))

(event Game|Damage|EventAnyDamage
  (params (Damage :type Float%20%28single-precision%29) (DamageType :type Damage%20Type%20Object%20Reference) (InstigatedBy :type Controller%20Object%20Reference) (DamageCauser :type Actor%20Object%20Reference))
  (CallFunction|GetDamages Damage)
  (Audio|PlaySoundatLocation "/Game/audio/Jab-SoundBible_com-1806727891_Cue.Jab-SoundBible_com-1806727891_Cue" (Transformation|GetActorLocation) "0, 0, 0" 1.0 1.0 0.0 0 0 0))

(fn ConstructionScript
  (bind _returnvalue (Rendering|Material|CreateDynamicMaterialInstance (Variables|Default|GetSkeletalMesh) 0 "/Game/Materials/M_Bird_Inst.M_Bird_Inst" "None" :!class /Script/Engine.PrimitiveComponent))
  (bind _output_get (Variables|Default|SetBirdMaterial _returnvalue))
  (Rendering|Material|SetVectorParameterValue _output_get "None" (Variables|Default|GetBirdColor) :!class /Script/Engine.MaterialInstanceDynamic)
  (Rendering|Material|SetMaterial (Variables|Default|GetSkeletalMesh) 0 (Variables|Default|GetBirdMaterial)))

(fn ChangeColor
  (params (Color :type Linear%20Color%20Structure))
  (bind (_r _g) (Math|Color|BreakColor Color))
  (bind _output_get (Variables|Default|SetBirdColor (Math|Color|MakeColor (+ _r (.R (Math|Color|BreakColor (Variables|Default|GetBirdColor)))) _g 0.0)))
  (Rendering|Material|SetVectorParameterValue (Variables|Default|GetBirdMaterial) "None" _output_get :!class /Script/Engine.MaterialInstanceDynamic)
  (Rendering|Material|SetMaterial (Variables|Default|GetSkeletalMesh) 0 (Variables|Default|GetBirdMaterial)))

(fn GetDamages
  (params (Damages :type Float%20%28single-precision%29))
  (bind _output_get (Variables|Default|SetHealth (- (Variables|Default|GetHealth) Damages)))
  (if (<= _output_get 0.0)
    (Utilities|FlowControl|DoOnce false
      (:Completed
        (Actor|DestroyActor)
        (bind _foundwidgets (Widget|GetAllWidgetsOfClass "/Game/Blueprints/UI/BP_PlayerHUD.BP_PlayerHUD_C" true))
        (Variables|/Game/Blueprints/UI/BP_PlayerHUD.BP_PlayerHUD_C|SetPoints (Utilities|Array|Get(acopy) _foundwidgets) (+ (Variables|/Game/Blueprints/UI/BP_PlayerHUD.BP_PlayerHUD_C|GetPoints (Utilities|Array|Get(acopy) _foundwidgets)) 10))))))

(fn FindDestination
  (bind _cages (Variables|Default|GetCages))
  (bind _returnvalue (Utilities|Array|Length _cages))
  (bind _returnvalue_2 (- _returnvalue 1))
  (bind _returnvalue_3 (Math|Random|RandomIntegerinRange 0 _returnvalue_2))
  (Variables|Default|SetHomeLocation (Transformation|GetActorLocation))
  (Variables|Default|SetDestination (Math|Random|RandomPointinBoundingBox (.Origin (Collision|GetActorBounds (Utilities|Array|Get(acopy) (Variables|Default|GetCages) (Variables|Default|GetCage)) false)) (.BoxExtent (Collision|GetActorBounds (Utilities|Array|Get(acopy) (Variables|Default|GetCages) (Variables|Default|GetCage)) false))))
  (bind _output_get (LocalVariables|SetNew%20Cage _returnvalue_3))
  (while (== (Variables|Default|GetCage) _output_get)
    (LocalVariables|SetNew%20Cage _returnvalue_3))
  (Variables|Default|SetCage (LocalVariables|GetNew%20Cage)))